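; Game state for an escape room that records a list of game events and persists it to a save slot.
; Saving passes the event data to a client save event, which writes it to a save game object; loading restores it from the slot.
; It also finds the newest checkpoint by scanning the events for the last entry of one type.
; Save and load print debug messages.
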(event Custom|Clients_SaveGame
  (params (SaveData :type S%20Escape%20Room%20Save%20Data%20Structure))
  (Variables|Default|SetSaveData SaveData)
  (bind _returnvalue (SaveGame|CreateSaveGameObject "/Game/EscapeRoom/Save/BP_EscapeRoomSaveGame.BP_EscapeRoomSaveGame_C"))
  (Variables|/Game/EscapeRoom/Save/BP_EscapeRoomSaveGame.BP_EscapeRoomSaveGame_C|SetSaveData _returnvalue (Variables|Default|GetSaveData))
  (bind _returnvalue_2 (SaveGame|SaveGametoSlot _returnvalue (Variables|Default|GetSaveSlot)))
  (Development|PrintString (Utilities|String|Append "Save Success: " (Utilities|String|ToString(Boolean) _returnvalue_2) " Events saved: " (Utilities|String|ToString(Integer) (Utilities|Array|Length (Utilities|Struct|BreakS_EscapeRoomSaveData (Variables|Default|GetSaveData))))) true true "(R=0.000000,G=0.660000,B=1.000000,A=1.000000)" 2e+01))

(fn ConstructionScript)

(fn SaveGame
  (CallFunction|ClientsSaveGame (Variables|Default|GetSaveData)))

(fn LoadGame
  (bind _returnvalue (SaveGame|DoesSaveGameExist (Variables|Default|GetSaveSlot)))
  (if _returnvalue
    (bind _returnvalue_2 (SaveGame|LoadGamefromSlot (Variables|Default|GetSaveSlot)))
    (bind _asbp_escape_room_save_game (Utilities|Casting|CastToBP_EscapeRoomSaveGame _returnvalue_2))
    (Variables|Default|SetSaveData (Variables|/Game/EscapeRoom/Save/BP_EscapeRoomSaveGame.BP_EscapeRoomSaveGame_C|GetSaveData _asbp_escape_room_save_game))
    (Development|PrintString (Utilities|String|Append "Events loaded: " (Utilities|String|ToString(Integer) (Utilities|Array|Length (Utilities|Struct|BreakS_EscapeRoomSaveData (Variables|/Game/EscapeRoom/Save/BP_EscapeRoomSaveGame.BP_EscapeRoomSaveGame_C|GetSaveData _asbp_escape_room_save_game))))) true true "(R=0.000000,G=0.660000,B=1.000000,A=1.000000)" 2e+01)))

(fn GetNewestCheckpointEventName
  (for _array_element (Utilities|Struct|BreakS_EscapeRoomSaveData (Variables|Default|GetSaveData))
    (if (Utilities|Enum|Equal(Enum) (.Type (Utilities|Struct|BreakS_Event _array_element)) "NewEnumerator1")
      (LocalVariables|SetLastCheckpointName (.EventName (Utilities|Struct|BreakS_Event _array_element)))))
  (return (LocalVariables|GetLastCheckpointName)))

(fn AddEvent
  (params (Event :type S%20Event%20Structure))
  (Utilities|Array|Add (Utilities|Struct|BreakS_EscapeRoomSaveData (Variables|Default|GetSaveData)) Event))