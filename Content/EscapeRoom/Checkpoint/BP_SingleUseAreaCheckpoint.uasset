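; Area checkpoint for the escape room that activates once, when an escape character first enters its Area volume.
; On BeginPlay the authority turns off the area's collision if the escape room save data already records an event with this checkpoint's name, and remote clients always turn it off.
; An overlap by the character calls Activate and then disables the collision, so triggering is server-only and single-use.
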(event OnComponentBeginOverlap(Area)
  (params (OverlappedComponent :type Primitive%20Component%20Object%20Reference) (OtherActor :type Actor%20Object%20Reference) (OtherComp :type Primitive%20Component%20Object%20Reference) (OtherBodyIndex :type Integer) (bFromSweep :type Boolean) (SweepResult :type Hit%20Result%20Structure%20%28by%20ref%29))
  (Utilities|Casting|CastToBP_EscapeCharacter OtherActor)
  (CallFunction|Activate)
  (Collision|SetCollisionEnabled (Variables|Default|GetArea) "NoCollision"))

(event EventBeginPlay
  (|CallParentFunction)
  (Networking|SwitchHasAuthority
    (:Authority
      (bind _state (Utilities|GetEscapeRoomState))
      (if (Utilities|Array|ContainsItem (Utilities|Struct|BreakS_EscapeRoomSaveData (Variables|/Game/EscapeRoom/BP_EscapeRoomGameState.BP_EscapeRoomGameState_C|GetSaveData _state)) (Utilities|Struct|MakeS_Event "NewEnumerator1" (Variables|Default|GetCheckpointName)))
        (Collision|SetCollisionEnabled (Variables|Default|GetArea) "NoCollision")))
    (:Remote
      (Collision|SetCollisionEnabled (Variables|Default|GetArea) "NoCollision"))))

(fn ConstructionScript
  (|CallParentFunction))