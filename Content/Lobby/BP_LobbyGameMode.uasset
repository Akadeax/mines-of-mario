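; Game mode for the escape room lobby, handling player joins, host save data and ready-to-start checks.
; On login it spawns and possesses a lobby character, flags the host via local control and binds to the player state's ready changes.
; Ready counts are compared with the player array to broadcast whether the game is startable.
; The save loaded at BeginPlay can be sent to clients through the lobby game state.
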(event EventBeginPlay
  (bind _returnvalue (SaveGame|DoesSaveGameExist (Variables|Default|GetSaveSlot)))
  (if _returnvalue
    (bind _returnvalue_2 (SaveGame|LoadGamefromSlot (Variables|Default|GetSaveSlot)))
    (bind _asbp_escape_room_save_game (Utilities|Casting|CastToBP_EscapeRoomSaveGame _returnvalue_2))
    (Variables|Default|SetHostSaveData (Variables|/Game/EscapeRoom/Save/BP_EscapeRoomSaveGame.BP_EscapeRoomSaveGame_C|GetSaveData _asbp_escape_room_save_game))))

(event EventPostLogin
  (params (NewPlayer :type Player%20Controller%20Object%20Reference))
  ;[0 0 0] When player logs in, spawn character and possess
  (Development|PrintString (Utilities|String|Append (PlayerState|GetPlayerName (Variables|/Script/Engine.Controller|GetPlayerState NewPlayer)) " Connected") true true "(R=0.000000,G=0.660000,B=1.000000,A=1.000000)" 6.0)
  (bind _returnvalue (Game|SpawnActorfromClass "/Game/Lobby/BP_LobbyCharacter.BP_LobbyCharacter_C" (Transformation|GetActorTransform) "AlwaysSpawn" "MultiplyWithRoot" NewPlayer 0))
  (Pawn|Possess NewPlayer _returnvalue)
  (bind _asbp_lobby_player_state (Utilities|Casting|CastToBP_LobbyPlayerState (Variables|/Script/Engine.Controller|GetPlayerState NewPlayer)))
  (Variables|/Game/Lobby/BP_LobbyPlayerState.BP_LobbyPlayerState_C|SetIsHost _asbp_lobby_player_state (Pawn|IsLocallyControlled _returnvalue))
  (EventDispatchers|BindEventtoReadyChanged _asbp_lobby_player_state (EventDispatchers|CreateEvent :!event AnyPlayeronReadyChanged)))

(fn ConstructionScript)

(fn CountReadyPlayers
  (for _array_element (Variables|/Script/Engine.GameStateBase|GetPlayerArray (Game|GetGameState))
    (bind _asbp_lobby_player_state (Utilities|Casting|CastToBP_LobbyPlayerState _array_element))
    (if (Variables|/Game/Lobby/BP_LobbyPlayerState.BP_LobbyPlayerState_C|GetReady _asbp_lobby_player_state)
      (Math|Integer|IncrementInt (LocalVariables|GetCurrentCount))))
  (return (LocalVariables|GetCurrentCount)))

(fn AnyPlayeronReadyChanged
  (params (NewReady :type Boolean))
  (bind _readycount (CallFunction|CountReadyPlayers))
  (Default|CallGameStartableChanged (== _readycount (Utilities|Array|Length (Variables|/Script/Engine.GameStateBase|GetPlayerArray (Game|GetGameState))))))

(fn SendHostSaveData
  (bind _asbp_lobby_game_state (Utilities|Casting|CastToBP_LobbyGameState (Game|GetGameState)))
  (Default|ClientsSetHostSaveData _asbp_lobby_game_state (Variables|Default|GetHostSaveData)))