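; BP_LobbyGameState is the lobby game state that holds the host's save data and derives the newest checkpoint name from it.
; The Clients_SetHostSaveData event stores the incoming save data and triggers CalculateFromSaveData.
; That function scans the save's event list and keeps the name of the last entry of one specific enum type as the newest checkpoint name.
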(event Custom|Clients_SetHostSaveData
  (params (SaveData :type S%20Escape%20Room%20Save%20Data%20Structure))
  (Variables|Default|SetHostSaveData SaveData)
  (CallFunction|CalculatefromSaveData))

(fn ConstructionScript)

(fn CalculatefromSaveData
  (for _array_element (Utilities|Struct|BreakS_EscapeRoomSaveData (Variables|Default|GetHostSaveData))
    (if (Utilities|Enum|Equal(Enum) (.Type (Utilities|Struct|BreakS_Event _array_element)) "NewEnumerator1")
      (LocalVariables|SetLast (.EventName (Utilities|Struct|BreakS_Event _array_element)))))
  (Variables|Default|SetNewestCheckpointName (LocalVariables|GetLast)))