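; Player controller for an escape room game that assigns each player one of two roles and prepares gameplay input.
; On BeginPlay it derives PlayerType by comparing the load subsystem's HostIsNavigator flag with HasAuthority, using the first type when they match and the second otherwise.
; If the Enhanced Input local player subsystem is valid, it adds the player mapping context and switches to game-only input.
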(event EventBeginPlay
  (bind _returnvalue (PlayerController|LocalPlayerSubsystems|GetEnhancedInputLocalPlayerSubsystem))
  (Variables|Default|SetPlayerType (select (not (Class|KismetMathLibrary|XORBoolean (Variables|/Script/MinesOfMario.EscapeRoomLoadSubsystem|GetHostIsNavigator (Subsystems|GetEscapeRoomLoadSubsystem)) (Ability|HasAuthority))) "NewEnumerator0" "NewEnumerator1"))
  (Utilities|IsValid _returnvalue
    (:Is%20Valid
      (Input|AddMappingContext _returnvalue "/Game/Player/Input/IMC_Player.IMC_Player" 0 "(bIgnoreAllPressedKeysUntilRelease=True,bForceImmediately=False,bNotifyUserSettings=False)")
      (Input|SetInputModeGameOnly self true))))

(fn ConstructionScript)